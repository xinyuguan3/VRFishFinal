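; Seagull actor that flies along the spline of a referenced track actor when play begins.
; A timeline, with its play rate set to the inverse of Duration, drives an alpha from BeginPlay.
; Each update maps that alpha to a distance along the spline and sets the seagull's world location and rotation to match.
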(event `self.ReceiveBeginPlay`
  (bind _returnvalue (`KismetMathLibrary.Lerp` 0.0 (`SplineComponent.GetSplineLength` (`/Game/Track.Spline` (`self.TrackReference`))) (`self.Alpha`)))
  (`TimelineComponent.SetPlayRate` (`self.Timeline_0`) (/ 1.0 (`self.Duration`)))
  (bind (_direction _alpha) (`Timeline|Timeline_0`)
    (:`Update`
      (set `self.Alpha` _alpha)
      (`self.K2_SetActorLocationAndRotation` (`SplineComponent.GetLocationAtDistanceAlongSpline` (`/Game/Track.Spline` (`self.TrackReference`)) _returnvalue "World") (`SplineComponent.GetRotationAtDistanceAlongSpline` (`/Game/Track.Spline` (`self.TrackReference`)) _returnvalue "World")))))

(event `self.ReceiveTick`
  (params (DeltaSeconds :type "Float (single-precision)")))

(fn `UserConstructionScript`)