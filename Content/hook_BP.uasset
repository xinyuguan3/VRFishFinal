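; hook_BP is an animated actor with two spinning halos and a bobbing cube; its gameplay role is not shown.
; Each Tick rotates Halo in yaw and Halo1 in pitch by frame-time-scaled deltas, combined with their relative rotations in opposite order.
; Tick also moves Cube along relative Z by Speed, using a two-second Delay to flip the sign of Speed and reverse its travel.
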(event `self.ReceiveTick`
  (params (DeltaSeconds :type "Float (single-precision)"))
  (bind _halo1 (`self.halo1`))
  (bind _halo (`self.halo`))
  (`|ExecutionSequence`
    (:`then_0`
      (`SceneComponent.K2_SetRelativeRotation` _halo (`KismetMathLibrary.ComposeRotators` (`SceneComponent.RelativeRotation` _halo) (* (`KismetMathLibrary.MakeRotator` 0.0 0.0 30.0) DeltaSeconds)) false false))
    (:`then_1`
      (`SceneComponent.K2_SetRelativeRotation` _halo1 (`KismetMathLibrary.ComposeRotators` (* (`KismetMathLibrary.MakeRotator` 0.0 -20.0 0.0) DeltaSeconds) (`SceneComponent.RelativeRotation` _halo1)) false false))
    (:`then_2`
      (`SceneComponent.K2_AddRelativeLocation` (`self.Cube`) (* (`KismetMathLibrary.MakeVector` 0.0 0.0 (`self.speed`)) DeltaSeconds) false false)
      (`KismetSystemLibrary.Delay` 2.0)
      (set `self.speed` (* (`self.speed`) -1.0)))))

(fn `UserConstructionScript`)